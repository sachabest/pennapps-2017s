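; VR gnome player Blueprint that calibrates the player's scale to the gnome skeleton and supplies tracking targets for its IK rig.
; Meshes stay hidden until calibration, triggered by right grip while left is held, or by T for testing without controllers.
; Calibration scales VROrigin by the ratio of skeleton hand span to controller span, then reveals both meshes.
; Tick then stores head and hand transforms relative to Mesh, whose pose FPSMesh follows.
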(event EventTick
  (params (DeltaSeconds :type Float%20%28single-precision%29))
  (bind _mesh (Variables|Character|GetMesh))
  (bind _returnvalue (Transformation|GetWorldTransform _mesh))
  (bind _returnvalue_2 (Math|Transform|InvertTransform _returnvalue))
  ;[1 1 1] Waits For Scale To Be Calibrated Then Gets Target Transforms For IKN Rig
  (if (Variables|Default|GetIsCalibrated?)
    (Variables|Default|SetRHand (Math|Transform|ComposeTransforms (Transformation|GetWorldTransform (Variables|Default|GetRightMotionCtr)) _returnvalue_2))
    (Variables|Default|SetlHand (Math|Transform|ComposeTransforms (Transformation|GetWorldTransform (Variables|Default|GetLeftMotionCtr)) _returnvalue_2))
    (Variables|Default|SetHead (Math|Transform|ComposeTransforms (Transformation|GetWorldTransform (Variables|Default|GetFRCamera)) _returnvalue_2))))

(event EventBeginPlay
  (Rendering|SetVisibility (Variables|Default|GetFPS%20Mesh) false false)
  (Rendering|SetVisibility (Variables|Character|GetMesh) false false)
  (Class|HeadMountedDisplayFunctionLibrary|SetTrackingOrigin "Floor")
  (Class|HeadMountedDisplayFunctionLibrary|ResetOrientationandPosition 0.0 "OrientationAndPosition")
  (Variables|/Script/Engine.CameraComponent|SetbLockToHmd (Variables|Default|GetFRCamera) true))

(event Input|KeyboardEvents|MotionControllerLeftGrip1
  (params (Key :type Key%20Structure :default "AnyKey"))
  (bind _mesh (Variables|Character|GetMesh))
  (bind _vrorigin (Variables|Default|GetVROrigin))
  ;[1 1 1] Setting The Human To Gnome Skeleton World Scale And Enabling Meshes
  (:Pressed
    (Utilities|FlowControl|Gate true) ; enters at Open
  )
  (:Released
    (Utilities|FlowControl|Gate true) ; enters at Close
  ))

(event Input|KeyboardEvents|T
  (params (Key :type Key%20Structure :default "AnyKey"))
  (bind _mesh (Variables|Character|GetMesh))
  (bind _vrorigin (Variables|Default|GetVROrigin))
  ;[1 1 1] For testing without vr controllers
  (:Pressed
    (Utilities|FlowControl|Gate false :!label _label
      (:Exit
        ;[1 1 1] Setting The Human To Gnome Skeleton World Scale And Enabling Meshes
        (Class|HeadMountedDisplayFunctionLibrary|SetTrackingOrigin "Floor")
        (Class|HeadMountedDisplayFunctionLibrary|ResetOrientationandPosition 0.0 "OrientationAndPosition")
        (Variables|/Script/Engine.CameraComponent|SetbLockToHmd (Variables|Default|GetFRCamera) true)
        (Transformation|SetWorldScale3D _vrorigin (* (Transformation|GetWorldScale _vrorigin) (/ (Math|Float|Absolute(Float) (.y (- (.Location (Math|Transform|BreakTransform (Transformation|GetSocketTransform _mesh "LeftHand" "RTS_Actor"))) (.Location (Math|Transform|BreakTransform (Transformation|GetSocketTransform _mesh "RightHand" "RTS_Actor")))))) (Math|Float|Absolute(Float) (.y (- (.location (Math|Transform|ComposeTransforms (Transformation|GetWorldTransform (Variables|Default|GetLeftMotionCtr)) (Math|Transform|InvertTransform (Transformation|GetActorTransform)))) (.location (Math|Transform|ComposeTransforms (Transformation|GetWorldTransform (Variables|Default|GetRightMotionCtr)) (Math|Transform|InvertTransform (Transformation|GetActorTransform))))))))))
        (Variables|Default|SetIsCalibrated? true)
        (Rendering|SetVisibility (Variables|Default|GetFPS%20Mesh) true false)
        (Rendering|SetVisibility (Variables|Character|GetMesh) true false)
        (Development|PrintString "Calibration Done!" true true "(R=0.000000,G=0.660000,B=1.000000,A=1.000000)" 5.0))))
  (:Released
    (goto _label Close)))

(event Input|KeyboardEvents|MotionControllerRightGrip1
  (params (Key :type Key%20Structure :default "AnyKey"))
  (bind _mesh (Variables|Character|GetMesh))
  (bind _vrorigin (Variables|Default|GetVROrigin))
  ;[1 1 1] Setting The Human To Gnome Skeleton World Scale And Enabling Meshes
  (:Pressed
    (Utilities|FlowControl|Gate true :!label _label
      (:Exit
        (Class|HeadMountedDisplayFunctionLibrary|SetTrackingOrigin "Floor")
        (Class|HeadMountedDisplayFunctionLibrary|ResetOrientationandPosition 0.0 "OrientationAndPosition")
        (Variables|/Script/Engine.CameraComponent|SetbLockToHmd (Variables|Default|GetFRCamera) true)
        (Transformation|SetWorldScale3D _vrorigin (* (Transformation|GetWorldScale _vrorigin) (/ (Math|Float|Absolute(Float) (.y (- (.Location (Math|Transform|BreakTransform (Transformation|GetSocketTransform _mesh "LeftHand" "RTS_Actor"))) (.Location (Math|Transform|BreakTransform (Transformation|GetSocketTransform _mesh "RightHand" "RTS_Actor")))))) (Math|Float|Absolute(Float) (.y (- (.location (Math|Transform|ComposeTransforms (Transformation|GetWorldTransform (Variables|Default|GetLeftMotionCtr)) (Math|Transform|InvertTransform (Transformation|GetActorTransform)))) (.location (Math|Transform|ComposeTransforms (Transformation|GetWorldTransform (Variables|Default|GetRightMotionCtr)) (Math|Transform|InvertTransform (Transformation|GetActorTransform))))))))))
        (Variables|Default|SetIsCalibrated? true)
        (Rendering|SetVisibility (Variables|Default|GetFPS%20Mesh) true false)
        (Rendering|SetVisibility (Variables|Character|GetMesh) true false)
        (Development|PrintString "Calibration Done!" true true "(R=0.000000,G=0.660000,B=1.000000,A=1.000000)" 5.0))))
  (:Released
    (goto _label Close)))

(fn ConstructionScript
  (Class|SkinnedMeshComponent|SetMasterPoseComponent (Variables|Default|GetFPS%20Mesh) (Variables|Character|GetMesh)))